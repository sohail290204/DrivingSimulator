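; BP_Car_Hatchback_Bot is a bot-driven hatchback that drives forward by itself and brakes for obstacles.
; A looping timer started on BeginPlay keeps the vehicle movement component at full throttle, with no steering logic in this graph.
; The AccidentCheck_0 trigger applies the brake when a component tagged Car, Playercar or Stop enters it and releases it when any such component leaves, without counting remaining overlaps.
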(event OnComponentBeginOverlap(AccidentCheck_0)
  (params (OverlappedComponent :type Primitive%20Component%20Object%20Reference) (OtherActor :type Actor%20Object%20Reference) (OtherComp :type Primitive%20Component%20Object%20Reference) (OtherBodyIndex :type Integer) (bFromSweep :type Boolean) (SweepResult :type Hit%20Result%20Structure%20%28by%20ref%29))
  (if (Math|Boolean|ORBoolean (Components|ComponentHasTag OtherComp "Car") (Components|ComponentHasTag OtherComp "Playercar") (Components|ComponentHasTag OtherComp "Stop"))
    (Class|ChaosVehicleMovementComponent|SetBrakeInput (Variables|Default|GetVehicleMovementComponent) 2e+01)))

(event OnComponentEndOverlap(AccidentCheck_0)
  (params (OverlappedComponent :type Primitive%20Component%20Object%20Reference) (OtherActor :type Actor%20Object%20Reference) (OtherComp :type Primitive%20Component%20Object%20Reference) (OtherBodyIndex :type Integer))
  (if (Math|Boolean|ORBoolean (Components|ComponentHasTag OtherComp "Car") (Components|ComponentHasTag OtherComp "Stop") (Components|ComponentHasTag OtherComp "Playercar"))
    (Class|ChaosVehicleMovementComponent|SetBrakeInput (Variables|Default|GetVehicleMovementComponent) 0.0)))

(event Custom|CustomEvent
  (Class|ChaosVehicleMovementComponent|SetThrottleInput (Variables|Default|GetVehicleMovementComponent) 1.0))

(event EventBeginPlay
  (Utilities|Time|SetTimerbyEvent (delegate Custom|CustomEvent) 0.01 true))

(event Collision|EventActorBeginOverlap
  (params (OtherActor :type Actor%20Object%20Reference)))

(event EventTick
  (params (DeltaSeconds :type Float%20%28single-precision%29)))

(fn ConstructionScript
  (|CallParentFunction))