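; SUV car Blueprint for an endless runner that handles crashes with other cars.
; When its AccidentCheck component overlaps a component tagged "Car", it calls DisableInput and shows the EndScreen widget, creating it only if no valid instance exists.
; After a short delay, it removes the widget and opens the EndlessRunner level.
; The construction script only calls its parent, and the other stock events are disabled placeholders.
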(event OnComponentBeginOverlap(AccidentCheck)
  (params (OverlappedComponent :type Primitive%20Component%20Object%20Reference) (OtherActor :type Actor%20Object%20Reference) (OtherComp :type Primitive%20Component%20Object%20Reference) (OtherBodyIndex :type Integer) (bFromSweep :type Boolean) (SweepResult :type Hit%20Result%20Structure%20%28by%20ref%29))
  (if (Components|ComponentHasTag OtherComp "Car")
    (Input|DisableInput 0)
    (bind _endscreen_widget (Variables|Default|GetEndscreen%20Widget)
      (:then
        (UserInterface|Viewport|AddtoViewport _endscreen_widget 0))
      (:else
        (bind _returnvalue (UserInterface|CreateWidget "/Game/UI/EndScreen.EndScreen_C"))
        (bind _output_get (Variables|Default|SetEndscreen%20Widget _returnvalue))
        (UserInterface|Viewport|AddtoViewport _output_get 0)))
    (Utilities|FlowControl|Delay 5.0)
    (bind _endscreen_widget_2 (Variables|Default|GetEndscreen%20Widget)
      (:then
        (Widget|RemovefromParent _endscreen_widget_2)
        (Game|OpenLevel(byObjectReference) "/Game/Levels/EndlessRunner_Lvl.EndlessRunner_Lvl"))
      (:else))))

(event EventBeginPlay
  (|CallParentFunction) ; This node is disabled and will not be called.\nDrag off pins to build functionality.
)

(event Collision|EventActorBeginOverlap
  (params (OtherActor :type Actor%20Object%20Reference)))

(event EventTick
  (params (DeltaSeconds :type Float%20%28single-precision%29)))

(fn ConstructionScript
  (|CallParentFunction))