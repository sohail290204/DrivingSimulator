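; Game mode for an endless-runner driving game that builds the road and spawns the player's car.
; BeginPlay optionally plays music and possesses the saved car choice, creating missing save slots, then lays the first road piece.
; Each SpawnRoad call randomly chains a piece straight, right or left from cached arrow locations, adding the current floor's yaw.
; It marks the previous piece with a matching direction actor and spawns cars on the new one.
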(event Custom|SpawnRoad
  (Variables|Default|SetDirection (Math|Random|RandomIntegerinRange 0 2))
  (Variables|Default|SetDirection_Rotation (Math|Random|RandomIntegerinRange 0 1))
  (bind _returnvalue (Game|SpawnActorfromClass "/Game/Assets/Road/Bp_StraightRoad.Bp_StraightRoad_C" (Math|Transform|MakeTransform (Utilities|Select :Index (Variables|Default|GetDirection) :Option%200 (Variables|Default|GetLocation%20Straight) :Option%201 (Variables|Default|GetLocation%20Right) :Option%202 (Variables|Default|GetLocation%20Left)) (Math|Rotator|MakeRotator (.roll (Utilities|Select :Index (Variables|Default|GetDirection) :Option%200 "0, 0, 0" :Option%201 (Variables|Default|GetRotation%20Right) :Option%202 (Variables|Default|GetRotation%20Left))) (.pitch (Utilities|Select :Index (Variables|Default|GetDirection) :Option%200 "0, 0, 0" :Option%201 (Variables|Default|GetRotation%20Right) :Option%202 (Variables|Default|GetRotation%20Left))) (+ (.yaw (Utilities|Select :Index (Variables|Default|GetDirection) :Option%200 "0, 0, 0" :Option%201 (Variables|Default|GetRotation%20Right) :Option%202 (Variables|Default|GetRotation%20Left))) (.yaw (Transformation|GetActorRotation (Variables|Default|GetFloor))))) "7.000000,7.000000,7.000000") "AlwaysSpawn" "MultiplyWithRoot" 0 0))
  (Utilities|FlowControl|Sequence
    (:then_1
      (switch int (Variables|Default|GetDirection)
        (:0
          (Game|SpawnActorfromClass "/Game/Assets/StopSign/Straight.Straight_C" (Transformation|GetWorldTransform (Variables|/Game/Assets/Road/Bp_StraightRoad.Bp_StraightRoad_C|GetStraightStopSign (Variables|Default|GetFloor))) "AlwaysSpawn" "MultiplyWithRoot" 0 0))
        (:1
          (Game|SpawnActorfromClass "/Game/Assets/StopSign/Right.Right_C" (Transformation|GetWorldTransform (Variables|/Game/Assets/Road/Bp_StraightRoad.Bp_StraightRoad_C|GetRightStopSign (Variables|Default|GetFloor))) "AlwaysSpawn" "MultiplyWithRoot" 0 0))
        (:2
          (Game|SpawnActorfromClass "/Game/Assets/StopSign/Left.Left_C" (Transformation|GetWorldTransform (Variables|/Game/Assets/Road/Bp_StraightRoad.Bp_StraightRoad_C|GetLeftStopSign (Variables|Default|GetFloor))) "AlwaysSpawn" "MultiplyWithRoot" 0 0)))
      (Variables|Default|SetFloor _returnvalue)
      (Variables|Default|SetLocation%20Right (Transformation|GetWorldLocation (Variables|/Game/Assets/Road/Bp_StraightRoad.Bp_StraightRoad_C|GetArrowRight _returnvalue)))
      (Variables|Default|SetLocation%20Left (Transformation|GetWorldLocation (Variables|/Game/Assets/Road/Bp_StraightRoad.Bp_StraightRoad_C|GetArrowLeft _returnvalue)))
      (Variables|Default|SetLocation%20Straight (Transformation|GetWorldLocation (Variables|/Game/Assets/Road/Bp_StraightRoad.Bp_StraightRoad_C|GetArrowStraight _returnvalue))))
    (:then_3
      (Default|SpawnCars _returnvalue))))

(event Custom|SpawnPlayer
  (bind _returnvalue (SaveGame|DoesSaveGameExist "CarGame" :!label _label))
  (if _returnvalue
    (bind _returnvalue_2 (SaveGame|LoadGamefromSlot "CarGame"))
    (bind _ascar_driving_save_game (Utilities|Casting|CastToCarDrivingSaveGame _returnvalue_2))
    (Utilities|IsValid _ascar_driving_save_game
      (:Is%20Valid
        (Variables|Default|SetCar%20Number (Variables|/Game/SaveGame/CarDrivingSaveGame.CarDrivingSaveGame_C|GetCarNumber _ascar_driving_save_game))
        (switch int (Variables|Default|GetCar%20Number)
          (:0
            (bind _returnvalue_3 (Game|SpawnActorfromClass "/Game/BP_Car/Car_Hatchback/BP_Car_Hatchback.BP_Car_Hatchback_C" (Variables|Default|GetStartLocation) "Undefined" "MultiplyWithRoot" 0 0))
            (Variables|Default|SetSpawnedPlayerCarRef _returnvalue_3)
            (Pawn|Possess (Game|GetPlayerController 0) _returnvalue_3))
          (:1
            (bind _returnvalue_4 (Game|SpawnActorfromClass "/Game/BP_Car/Car_PickUp/BP_Car_PickUp.BP_Car_PickUp_C" (Variables|Default|GetStartLocation) "Undefined" "MultiplyWithRoot" 0 0))
            (Variables|Default|SetSpawnedPlayerCarRef _returnvalue_4)
            (Pawn|Possess (Game|GetPlayerController 0) _returnvalue_4))
          (:2
            (bind _returnvalue_5 (Game|SpawnActorfromClass "/Game/BP_Car/Car_SUV/BP_Car_SUV.BP_Car_SUV_C" (Variables|Default|GetStartLocation) "Undefined" "MultiplyWithRoot" 0 0))
            (Variables|Default|SetSpawnedPlayerCarRef _returnvalue_5)
            (Pawn|Possess (Game|GetPlayerController 0) _returnvalue_5))
          (:3
            (bind _returnvalue_6 (Game|SpawnActorfromClass "/Game/BP_Car/Car_SportsCar/BP_Car_SportsCar.BP_Car_SportsCar_C" (Variables|Default|GetStartLocation) "Undefined" "MultiplyWithRoot" 0 0))
            (Variables|Default|SetSpawnedPlayerCarRef _returnvalue_6)
            (Pawn|Possess (Game|GetPlayerController 0) _returnvalue_6)))))
    (else
      (bind _returnvalue_7 (SaveGame|CreateSaveGameObject "/Game/SaveGame/CarDrivingSaveGame.CarDrivingSaveGame_C"))
      (SaveGame|SaveGametoSlot _returnvalue_7 "CarGame")
      (goto _label))))

(event Custom|PlaySound
  (bind _returnvalue (SaveGame|DoesSaveGameExist "BG_Music" :!label _label))
  (if _returnvalue
    (bind _returnvalue_2 (SaveGame|LoadGamefromSlot "BG_Music"))
    (bind _ascar_driving_save_game (Utilities|Casting|CastToCarDrivingSaveGame _returnvalue_2))
    (Utilities|IsValid _ascar_driving_save_game
      (:Is%20Valid
        (if (Variables|/Game/SaveGame/CarDrivingSaveGame.CarDrivingSaveGame_C|GetBG_Sound _ascar_driving_save_game)
          (Audio|PlaySound2D "/Game/Assets/Sounds/MainBackgroundMusic_Cue.MainBackgroundMusic_Cue" 1.0 1.0 0.0 0 0))))
    (else
      (bind _returnvalue_3 (SaveGame|CreateSaveGameObject "/Game/SaveGame/CarDrivingSaveGame.CarDrivingSaveGame_C"))
      (SaveGame|SaveGametoSlot _returnvalue_3 "BG_Music")
      (goto _label))))

(event EventBeginPlay
  (CallFunction|PlaySound)
  (CallFunction|SpawnPlayer)
  (bind _returnvalue (Actor|GetActorOfClass "/Game/Assets/Road/Bp_StraightRoad.Bp_StraightRoad_C"))
  (Variables|Default|SetLocation%20Straight (Transformation|GetWorldLocation (Variables|/Game/Assets/Road/Bp_StraightRoad.Bp_StraightRoad_C|GetArrowStraight _returnvalue)))
  (bind _returnvalue_2 (Game|SpawnActorfromClass "/Game/Assets/Road/Bp_StraightRoad.Bp_StraightRoad_C" (Math|Transform|MakeTransform (Variables|Default|GetLocation%20Straight) "0, 0, 0" "7.000000,7.000000,7.000000") "AlwaysSpawn" "MultiplyWithRoot" 0 0))
  (Variables|Default|SetFloor _returnvalue_2)
  (Utilities|FlowControl|Sequence
    (:then_0
      (Default|SpawnCars _returnvalue_2)
      (Variables|Default|SetLocation%20Right (Transformation|GetWorldLocation (Variables|/Game/Assets/Road/Bp_StraightRoad.Bp_StraightRoad_C|GetArrowRight _returnvalue_2)))
      (Variables|Default|SetLocation%20Left (Transformation|GetWorldLocation (Variables|/Game/Assets/Road/Bp_StraightRoad.Bp_StraightRoad_C|GetArrowLeft _returnvalue_2)))
      (Variables|Default|SetLocation%20Straight (Transformation|GetWorldLocation (Variables|/Game/Assets/Road/Bp_StraightRoad.Bp_StraightRoad_C|GetArrowStraight _returnvalue_2)))
      (Variables|Default|SetDirection 0))))

(event EventTick
  (params (DeltaSeconds :type Float%20%28single-precision%29)))

(fn ConstructionScript)