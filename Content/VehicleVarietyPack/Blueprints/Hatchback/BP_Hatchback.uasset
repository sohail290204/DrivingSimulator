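; BP_Hatchback is a player-drivable hatchback vehicle Blueprint from the Vehicle Variety Pack.
; Movement axes and the Handbrake action feed throttle, steering and handbrake input straight into the VehicleMovement component.
; Look axes drive controller yaw and pitch, with the pitch value negated.
; The construction script is empty, and the graphs hold only this input forwarding.
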(event Input|ActionEvents|InputActionHandbrake
  (params (Key :type Key%20Structure :default "None"))
  (bind _vehiclemovement (Variables|Default|GetVehicleMovement))
  (:Pressed
    (CallFunction|SetHandbrakeInput _vehiclemovement true))
  (:Released
    (CallFunction|SetHandbrakeInput _vehiclemovement false)))

(event Input|AxisEvents|InputAxisMoveForward
  (params (AxisValue :type Float%20%28double-precision%29))
  (CallFunction|SetThrottleInput (Variables|Default|GetVehicleMovement) AxisValue))

(event Input|AxisEvents|InputAxisMoveRight
  (params (AxisValue :type Float%20%28double-precision%29))
  (CallFunction|SetSteeringInput (Variables|Default|GetVehicleMovement) AxisValue))

(event Input|AxisEvents|InputAxisLookUp
  (params (AxisValue :type Float%20%28double-precision%29))
  (Pawn|Input|AddControllerPitchInput (* AxisValue -1.0)))

(event Input|AxisEvents|InputAxisLookRight
  (params (AxisValue :type Float%20%28double-precision%29))
  (Pawn|Input|AddControllerYawInput AxisValue))

(fn ConstructionScript)