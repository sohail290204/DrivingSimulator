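; Straight road segment actor for a car game with a road that spawns as the car drives.
; It caches the Bp_CarGameModeBase on BeginPlay and calls its SpawnRoad when a Car-tagged component enters SpawnBox.
; Three destroy boxes each remove the segment after a short delay once a Car-tagged component leaves them.
; Unconnected Collision calls on Right, Left and Straight child actors never run.
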(event OnComponentBeginOverlap(SpawnBox)
  (params (OverlappedComponent :type Primitive%20Component%20Object%20Reference) (OtherActor :type Actor%20Object%20Reference) (OtherComp :type Primitive%20Component%20Object%20Reference) (OtherBodyIndex :type Integer) (bFromSweep :type Boolean) (SweepResult :type Hit%20Result%20Structure%20%28by%20ref%29))
  (if (Components|ComponentHasTag OtherComp "Car")
    (Default|SpawnRoad (Variables|Default|GetAs%20Bp%20Car%20Game%20Mode%20Base))))

(event OnComponentEndOverlap(DestroyBox2)
  (params (OverlappedComponent :type Primitive%20Component%20Object%20Reference) (OtherActor :type Actor%20Object%20Reference) (OtherComp :type Primitive%20Component%20Object%20Reference) (OtherBodyIndex :type Integer))
  (if (Components|ComponentHasTag OtherComp "Car")
    (Utilities|FlowControl|Delay 5.0)
    (Actor|DestroyActor)))

(event OnComponentEndOverlap(DestroyBox1)
  (params (OverlappedComponent :type Primitive%20Component%20Object%20Reference) (OtherActor :type Actor%20Object%20Reference) (OtherComp :type Primitive%20Component%20Object%20Reference) (OtherBodyIndex :type Integer))
  (if (Components|ComponentHasTag OtherComp "Car")
    (Utilities|FlowControl|Delay 5.0)
    (Actor|DestroyActor)))

(event OnComponentEndOverlap(DestroyBox)
  (params (OverlappedComponent :type Primitive%20Component%20Object%20Reference) (OtherActor :type Actor%20Object%20Reference) (OtherComp :type Primitive%20Component%20Object%20Reference) (OtherBodyIndex :type Integer))
  (if (Components|ComponentHasTag OtherComp "Car")
    (Utilities|FlowControl|Delay 5.0)
    (Actor|DestroyActor)))

(event Collision|EventActorBeginOverlap
  (params (OtherActor :type Actor%20Object%20Reference)))

(event EventTick
  (params (DeltaSeconds :type Float%20%28single-precision%29)))

(event EventBeginPlay
  (Utilities|FlowControl|Sequence
    (:then_0
      (bind _asbp_car_game_mode_base (Utilities|Casting|CastToBp_CarGameModeBase (Game|GetGameMode)))
      (Variables|Default|SetAs%20Bp%20Car%20Game%20Mode%20Base _asbp_car_game_mode_base))))

(fn ConstructionScript)