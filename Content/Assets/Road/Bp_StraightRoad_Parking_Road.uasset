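; Straight parking road tile for the driving game that spawns traffic and tracks the player car's parking range.
; Leaving a destroy box reveals a blocking container, then destroys the tile after a delay.
; SpawnCars starts three looping lane timers that sphere-trace before spawning random cars at random offsets.
; Range triggers set parking flags on the hatchback; next-road spawning and parking-success logic are disconnected, though BeginPlay still caches the active game mode.
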(event OnComponentBeginOverlap(SpawnBox)
  (params (OverlappedComponent :type Primitive%20Component%20Object%20Reference) (OtherActor :type Actor%20Object%20Reference) (OtherComp :type Primitive%20Component%20Object%20Reference) (OtherBodyIndex :type Integer) (bFromSweep :type Boolean) (SweepResult :type Hit%20Result%20Structure%20%28by%20ref%29))
  ;[0.15 0.15 0.15 0.5] Spawn New Floor
)

(event OnComponentBeginOverlap(PlayerInsideRange)
  (params (OverlappedComponent :type Primitive%20Component%20Object%20Reference) (OtherActor :type Actor%20Object%20Reference) (OtherComp :type Primitive%20Component%20Object%20Reference) (OtherBodyIndex :type Integer) (bFromSweep :type Boolean) (SweepResult :type Hit%20Result%20Structure%20%28by%20ref%29))
  (if (== OtherActor (Game|Player|GetPlayerPawn 0))
    (bind _asbp_car_hatchback (Utilities|Casting|CastToBP_Car_Hatchback OtherActor))
    (Variables|/Game/BP_Car/Car_Hatchback/BP_Car_Hatchback.BP_Car_Hatchback_C|SetPlayer%20In%20Parking%20range _asbp_car_hatchback true)))

(event OnComponentEndOverlap(DestroyBox2)
  (params (OverlappedComponent :type Primitive%20Component%20Object%20Reference) (OtherActor :type Actor%20Object%20Reference) (OtherComp :type Primitive%20Component%20Object%20Reference) (OtherBodyIndex :type Integer))
  (bind _container_lowpoly1 (Variables|Default|GetContainer_LowPoly1))
  ;[0.15 0.15 0.15 0.5] Destroy Floor
  (if (Components|ComponentHasTag OtherComp "Playercar")
    (Development|SetHiddeninGame _container_lowpoly1 false false)
    (Collision|SetCollisionEnabled _container_lowpoly1 "QueryAndPhysics")
    (Utilities|FlowControl|Delay 3.0)
    (Actor|DestroyActor)))

(event OnComponentEndOverlap(DestroyBox1)
  (params (OverlappedComponent :type Primitive%20Component%20Object%20Reference) (OtherActor :type Actor%20Object%20Reference) (OtherComp :type Primitive%20Component%20Object%20Reference) (OtherBodyIndex :type Integer))
  (bind _container_lowpoly3 (Variables|Default|GetContainer_LowPoly3))
  ;[0.15 0.15 0.15 0.5] Destroy Floor
  (if (Components|ComponentHasTag OtherComp "Playercar")
    (Development|SetHiddeninGame _container_lowpoly3 false false)
    (Collision|SetCollisionEnabled _container_lowpoly3 "QueryAndPhysics")
    (Utilities|FlowControl|Delay 3.0)
    (Actor|DestroyActor)))

(event OnComponentEndOverlap(DestroyBox)
  (params (OverlappedComponent :type Primitive%20Component%20Object%20Reference) (OtherActor :type Actor%20Object%20Reference) (OtherComp :type Primitive%20Component%20Object%20Reference) (OtherBodyIndex :type Integer))
  (bind _container_lowpoly2 (Variables|Default|GetContainer_LowPoly2))
  ;[0.15 0.15 0.15 0.5] Destroy Floor
  (if (Components|ComponentHasTag OtherComp "Playercar")
    (Development|SetHiddeninGame _container_lowpoly2 false false)
    (Collision|SetCollisionEnabled _container_lowpoly2 "QueryAndPhysics")
    (Utilities|FlowControl|Delay 3.0)
    (Actor|DestroyActor)))

(event OnComponentEndOverlap(PlayerInsideRange)
  (params (OverlappedComponent :type Primitive%20Component%20Object%20Reference) (OtherActor :type Actor%20Object%20Reference) (OtherComp :type Primitive%20Component%20Object%20Reference) (OtherBodyIndex :type Integer))
  (if (== OtherActor (Game|Player|GetPlayerPawn 0))
    (bind _asbp_car_hatchback (Utilities|Casting|CastToBP_Car_Hatchback OtherActor))
    (Variables|/Game/BP_Car/Car_Hatchback/BP_Car_Hatchback.BP_Car_Hatchback_C|SetPlayer%20In%20Parking%20range _asbp_car_hatchback false)))

(event OnComponentBeginOverlap(PlayerOutsideRange)
  (params (OverlappedComponent :type Primitive%20Component%20Object%20Reference) (OtherActor :type Actor%20Object%20Reference) (OtherComp :type Primitive%20Component%20Object%20Reference) (OtherBodyIndex :type Integer) (bFromSweep :type Boolean) (SweepResult :type Hit%20Result%20Structure%20%28by%20ref%29))
  (if (== OtherActor (Game|Player|GetPlayerPawn 0))
    (bind _asbp_car_hatchback (Utilities|Casting|CastToBP_Car_Hatchback OtherActor))
    (Variables|/Game/BP_Car/Car_Hatchback/BP_Car_Hatchback.BP_Car_Hatchback_C|SetPlayer%20outside%20Parking%20range _asbp_car_hatchback true)))

(event OnComponentEndOverlap(PlayerOutsideRange)
  (params (OverlappedComponent :type Primitive%20Component%20Object%20Reference) (OtherActor :type Actor%20Object%20Reference) (OtherComp :type Primitive%20Component%20Object%20Reference) (OtherBodyIndex :type Integer))
  (if (== OtherActor (Game|Player|GetPlayerPawn 0))
    (bind _asbp_car_hatchback (Utilities|Casting|CastToBP_Car_Hatchback OtherActor))
    (Variables|/Game/BP_Car/Car_Hatchback/BP_Car_Hatchback.BP_Car_Hatchback_C|SetPlayer%20outside%20Parking%20range _asbp_car_hatchback false)))

(event Custom|Spawn%20Cars
  (params (NewParam :type Integer))
  ;[0.15 0.15 0.15 0.5] Spawn Cars
  (Utilities|FlowControl|Sequence
    (:then_0
      (CallFunction|Car1))
    (:then_1
      (CallFunction|Car2))
    (:then_2
      (CallFunction|Car3))))

(event Custom|CustomEvent_15
  ;[0.15 0.15 0.15 0.5] Spawn car at lane 3
  (CallFunction|SphereCheck))

(event Custom|Car3
  ;[0.15 0.15 0.15 0.5] Spawn car at lane 3
  (Utilities|Time|SetTimerbyEvent (delegate Custom|CustomEvent_15) 3.0 true))

(event Custom|Car1
  ;[0.15 0.15 0.15 0.5] Spawn car at lane 1
  (Utilities|Time|SetTimerbyEvent (delegate Custom|CustomEvent) 3.0 true))

(event Custom|SphereCheck
  (bind _cars (Variables|Default|Getcars))
  (bind _spawn_cars_left (Variables|Default|GetSpawn%20Cars%20Left))
  (bind _spawn_cars_left_2 (Variables|Default|GetSpawn%20Cars%20Left))
  (bind _returnvalue (Transformation|GetWorldTransform _spawn_cars_left))
  ;[0.15 0.15 0.15 0.5] Spawn car at lane 3
  (bind _outhit (Collision|SphereTraceByChannel (Transformation|GetWorldLocation _spawn_cars_left_2) (Transformation|GetWorldLocation _spawn_cars_left_2) 5e+03 "TraceTypeQuery1" false 0 "None" false "(R=1.000000,G=0.000000,B=0.000000,A=1.000000)" "(R=0.000000,G=1.000000,B=0.000000,A=1.000000)" 2e+01))
  (if (.bBlockingHit (Collision|BreakHitResult _outhit))
    (if (== (.HitActor (Collision|BreakHitResult _outhit)) (Game|Player|GetPlayerPawn 0))
      (Development|PrintString "Hello")
      (else
        (Game|SpawnActorfromClass (Utilities|Array|Get(acopy) _cars (Math|Random|RandomIntegerinRange 0 (Utilities|Array|Length _cars))) (Math|Transform|MakeTransform (+ (.location _returnvalue) (Math|Vector|MakeVector (Utilities|Array|Get(acopy) (Variables|Default|GetSpawnLocation) (Math|Random|RandomIntegerinRange 0 4)) 0.0 0.0)) (.rotation _returnvalue) "1.000000,1.000000,1.000000") "AdjustIfPossibleButDontSpawnIfColliding" "MultiplyWithRoot" 0 0)))))

(event Custom|Car%202
  ;[0.15 0.15 0.15 0.5] Spawn car at lane 2
  (Utilities|Time|SetTimerbyEvent (delegate Custom|CustomEvent_12) 3.0 true))

(event Custom|CustomEvent
  (bind _spawn_cars_straight (Variables|Default|GetSpawn%20Cars%20Straight))
  (bind _spawn_cars_straight_2 (Variables|Default|GetSpawn%20Cars%20Straight))
  (bind _cars (Variables|Default|Getcars))
  (bind _returnvalue (Transformation|GetWorldTransform _spawn_cars_straight_2))
  ;[0.15 0.15 0.15 0.5] Spawn car at lane 1
  (bind _outhit (Collision|SphereTraceByChannel (Transformation|GetWorldLocation _spawn_cars_straight) (Transformation|GetWorldLocation _spawn_cars_straight) 5e+03 "TraceTypeQuery1" false 0 "None" false "(R=1.000000,G=0.000000,B=0.000000,A=1.000000)" "(R=0.000000,G=1.000000,B=0.000000,A=1.000000)" 2e+01))
  (if (.bBlockingHit (Collision|BreakHitResult _outhit))
    (if (not (== (.HitActor (Collision|BreakHitResult _outhit)) (Game|Player|GetPlayerPawn 0)))
      (Game|SpawnActorfromClass (Utilities|Array|Get(acopy) _cars (Math|Random|RandomIntegerinRange 0 (Utilities|Array|Length _cars))) (Math|Transform|MakeTransform (+ (.location _returnvalue) (Math|Vector|MakeVector (Utilities|Array|Get(acopy) (Variables|Default|GetSpawnLocation) (Math|Random|RandomIntegerinRange 0 4)) 0.0 0.0)) (.rotation _returnvalue) "1.000000,1.000000,1.000000") "AdjustIfPossibleButDontSpawnIfColliding" "MultiplyWithRoot" 0 0))))

(event Custom|CustomEvent_12
  (bind _cars (Variables|Default|Getcars))
  (bind _spawn_cars_right (Variables|Default|GetSpawn%20Cars%20Right))
  (bind _spawn_cars_right_2 (Variables|Default|GetSpawn%20Cars%20Right))
  (bind _returnvalue (Transformation|GetWorldTransform _spawn_cars_right_2))
  ;[0.15 0.15 0.15 0.5] Spawn car at lane 2
  (bind _outhit (Collision|SphereTraceByChannel (Transformation|GetWorldLocation _spawn_cars_right) (Transformation|GetWorldLocation _spawn_cars_right) 5e+03 "TraceTypeQuery1" false 0 "None" false "(R=1.000000,G=0.000000,B=0.000000,A=1.000000)" "(R=0.000000,G=1.000000,B=0.000000,A=1.000000)" 2e+01))
  (if (.bBlockingHit (Collision|BreakHitResult _outhit))
    (if (== (.HitActor (Collision|BreakHitResult _outhit)) (Game|Player|GetPlayerPawn 0))
      (Development|PrintString "Hello")
      (else
        (Game|SpawnActorfromClass (Utilities|Array|Get(acopy) _cars (Math|Random|RandomIntegerinRange 0 (Utilities|Array|Length _cars))) (Math|Transform|MakeTransform (+ (.location _returnvalue) (Math|Vector|MakeVector 0.0 (Utilities|Array|Get(acopy) (Variables|Default|GetSpawnLocation) (Math|Random|RandomIntegerinRange 0 4)) 0.0)) (.rotation _returnvalue) "1.000000,1.000000,1.000000") "AdjustIfPossibleButDontSpawnIfColliding" "MultiplyWithRoot" 0 0)))))

(event EventBeginPlay
  (bind _returnvalue (Game|GetGameMode))
  (bind _container_lowpoly (Variables|Default|GetContainer_LowPoly))
  ;[0.15 0.15 0.15 0.5] Begin Play
  (Utilities|FlowControl|Sequence
    (:then_0
      ;[0.15 0.15 0.15 0.5] Game Modes
      (Utilities|FlowControl|Delay 0.2)
      (bind _asdriving_game_instance (Utilities|Casting|CastToDrivingGameInstance (Game|GetGameInstance)))
      (if (Variables|/Game/SaveGame/DrivingGameInstance.DrivingGameInstance_C|GetBrakeFail _asdriving_game_instance)
        (bind _asbp_car_brake_fail_game_mode (Utilities|Casting|CastToBp_Car_BrakeFailGameMode _returnvalue))
        (Variables|Default|SetAs%20Bp%20Car%20Brake%20Fail%20Game%20Mode _asbp_car_brake_fail_game_mode)
        (elif (Variables|/Game/SaveGame/DrivingGameInstance.DrivingGameInstance_C|GetFuel_Save _asdriving_game_instance)
          (bind _asbp_car_save_fuel_game_mode (Utilities|Casting|CastToBp_Car_SaveFuel_GameMode _returnvalue))
          (Variables|Default|SetAs%20Bp%20Car%20Save%20Fuel%20Game%20Mode _asbp_car_save_fuel_game_mode)
          (elif (Variables|/Game/SaveGame/DrivingGameInstance.DrivingGameInstance_C|GetTimer _asdriving_game_instance)
            (bind _asbp_car_timer_game_mode (Utilities|Casting|CastToBp_Car_Timer_GameMode _returnvalue))
            (Variables|Default|SetAs%20Bp%20Car%20Timer%20Game%20Mode _asbp_car_timer_game_mode)
            (else
              (bind _asbp_car_endless_runner_game_mode (Utilities|Casting|CastToBp_Car_EndlessRunnerGameMode _returnvalue))
              (Variables|Default|SetAs%20Bp%20Car%20Endless%20Runner%20Game%20Mode _asbp_car_endless_runner_game_mode))))))
    (:then_2
      ;[0.15 0.15 0.15 0.5] Hide Containers
      (Development|SetHiddeninGame _container_lowpoly true false)
      (Collision|SetCollisionEnabled _container_lowpoly "NoCollision"))))

(fn ConstructionScript)